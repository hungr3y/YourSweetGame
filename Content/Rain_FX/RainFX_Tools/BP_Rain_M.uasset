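; Configurable rain effect actor that sets up its Rain particle component in the construction script, with no active runtime logic.
; RainType selects one of four presets for drop shape, spawn rate, speed, rotation and hit style, or keeps the current values.
; Values feed the effect's parameters, with length remapped inversely and lifetime derived from velocity.
; All presets share an Area reset to 1000, overriding the fourth preset's larger area.
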(event EventBeginPlay)

(event Collision|EventActorBeginOverlap
  (params (OtherActor :type Actor%20Object%20Reference)))

(event EventTick
  (params (DeltaSeconds :type Float%20%28single-precision%29)))

(fn ConstructionScript
  (bind _rain (Variables|Default|Getrain))
  (bind _rain_type (Variables|Default|GetRain_Type))
  (bind _rain_2 (Variables|Default|Getrain))
  (bind _rain_3 (Variables|Default|Getrain))
  (bind _rain_4 (Variables|Default|Getrain))
  (Utilities|FlowControl|Sequence
    (:then_0
      (if (Utilities|Enum|Equal(Enum) _rain_type "NewEnumerator1")
        (Variables|intensity|Setintensity 0.5)
        (Variables|Length|SetMin_Length 0.2)
        (Variables|Length|SetMax_Length 0.5)
        (Variables|Width|SetMin_Width 0.4)
        (Variables|Width|SetMax_Width 0.5)
        (Variables|intensity|SetSpawn_Rate 200)
        (Variables|Direction|SetMax_rot 1.0)
        (Variables|Direction|SetMin_rot -1.0)
        (Variables|Direction|Setvelocity 9e+02)
        (Variables|Hit_Drop|SetHit_Type 1)
        (Variables|Hit_Drop|SetHit_Scale 1.0)
        (Variables|Default|SetArea 1e+03 :!label _label)
        (Niagara|SetNiagaraVariable(Float) _rain_3 "int" (Variables|intensity|Getintensity) :!label _label_2)
        (Niagara|SetNiagaraVariable(Vector3) _rain_3 "color" (Math|Vector|MakeVector (.R (Utilities|Struct|BreakLinearColor (Variables|Default|GetColor))) (.G (Utilities|Struct|BreakLinearColor (Variables|Default|GetColor))) (.B (Utilities|Struct|BreakLinearColor (Variables|Default|GetColor)))))
        (Niagara|SetNiagaraVariable(Float) (Variables|Default|Getrain) "switch" (Math|Conversions|ToFloat(Integer) (Variables|Hit_Drop|GetHit_Type)))
        (Niagara|SetNiagaraVariable(Float) (Variables|Default|Getrain) "Rain_Intensity" (Math|Conversions|ToFloat(Integer) (Variables|intensity|GetSpawn_Rate)))
        (Niagara|SetNiagaraVariable(Float) _rain "lemin" (Math|Float|MapRangeClamped (Variables|Length|GetMin_Length) 0.0 1.0 1.0 -1.0))
        (Niagara|SetNiagaraVariable(Float) _rain "lemax" (Math|Float|MapRangeClamped (Variables|Length|GetMax_Length) 0.0 1.0 1.0 -1.0))
        (Niagara|SetNiagaraVariable(Float) _rain "wgmin" (Variables|Width|GetMin_Width))
        (Niagara|SetNiagaraVariable(Float) _rain "wgmax" (Variables|Width|GetMax_Width))
        (Niagara|SetNiagaraVariable(Float) _rain_2 "max_Rot" (Variables|Direction|GetMax_rot))
        (Niagara|SetNiagaraVariable(Float) _rain_2 "min_Rot" (Variables|Direction|GetMin_rot))
        (Niagara|SetNiagaraVariable(Float) _rain_4 "vel" (Variables|Direction|Getvelocity))
        (Niagara|SetNiagaraVariable(Float) _rain_4 "life" (Math|Float|MapRangeClamped (Variables|Direction|Getvelocity) 1e+02 1e+03 5.0 2.0))
        (Niagara|SetNiagaraVariable(Float) (Variables|Default|Getrain) "hitdropscale" (Variables|Hit_Drop|GetHit_Scale))
        (Niagara|SetNiagaraVariable(Float) (Variables|Default|Getrain) "Area" (Variables|Default|GetArea))))
    (:then_1
      (if (Utilities|Enum|Equal(Enum) _rain_type "NewEnumerator2")
        (Variables|intensity|Setintensity 0.7)
        (Variables|Length|SetMin_Length 0.5)
        (Variables|Length|SetMax_Length 1.0)
        (Variables|Width|SetMin_Width 0.35)
        (Variables|Width|SetMax_Width 0.45)
        (Variables|intensity|SetSpawn_Rate 600)
        (Variables|Direction|SetMax_rot 5.0)
        (Variables|Direction|SetMin_rot -5.0)
        (Variables|Direction|Setvelocity 1e+03)
        (Variables|Hit_Drop|SetHit_Type 2)
        (Variables|Hit_Drop|SetHit_Scale 0.6)
        (goto _label)))
    (:then_2
      (if (Utilities|Enum|Equal(Enum) _rain_type "NewEnumerator3")
        (Variables|intensity|Setintensity 1.0)
        (Variables|Length|SetMin_Length 0.2)
        (Variables|Length|SetMax_Length 1.0)
        (Variables|Width|SetMin_Width 0.4)
        (Variables|Width|SetMax_Width 0.5)
        (Variables|intensity|SetSpawn_Rate 1000)
        (Variables|Direction|SetMax_rot 1e+01)
        (Variables|Direction|SetMin_rot -1e+01)
        (Variables|Direction|Setvelocity 1.2e+03)
        (Variables|Hit_Drop|SetHit_Type 3)
        (Variables|Hit_Drop|SetHit_Scale 0.6)
        (goto _label)))
    (:then_3
      (if (Utilities|Enum|Equal(Enum) _rain_type "NewEnumerator4")
        (Variables|Default|SetArea 2.5e+03)
        (Variables|intensity|Setintensity 0.2)
        (Variables|Length|SetMin_Length 0.2)
        (Variables|Length|SetMax_Length 1.0)
        (Variables|Width|SetMin_Width 0.4)
        (Variables|Width|SetMax_Width 0.5)
        (Variables|intensity|SetSpawn_Rate 18000)
        (Variables|Direction|SetMax_rot 1e+01)
        (Variables|Direction|SetMin_rot -1e+01)
        (Variables|Direction|Setvelocity 1.2e+03)
        (Variables|Hit_Drop|SetHit_Type 3)
        (Variables|Hit_Drop|SetHit_Scale 0.6)
        (Variables|Default|SetColor "(R=0.341667,G=0.341667,B=0.341667,A=1.000000)")
        (goto _label)))
    (:then_4
      (if (Utilities|Enum|Equal(Enum) _rain_type "NewEnumerator0")
        (goto _label_2)))))